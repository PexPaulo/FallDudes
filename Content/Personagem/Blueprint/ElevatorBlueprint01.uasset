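; Elevator platform Blueprint that shuttles a static mesh endlessly between DownPos and UpPos, starting on BeginPlay.
; StartDown picks the starting end and one of two mirrored timelines, MoveElevator or Timeline.
; Each timeline's Blend track drives a transform lerp, of which only the world location is applied, without sweep.
; On finishing, the timeline pauses briefly, then runs in the opposite direction.
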(event `self.ReceiveBeginPlay`
  (if (`self.startDown`)
    (`SceneComponent.K2_SetWorldLocation` (`self.StaticMeshComponent0`) (.location (`self.DownPos`)) false false)
    (bind (_direction _blend) (`Timeline|MoveElevator` :!label _label)
      (:`Update`
        (`SceneComponent.K2_SetWorldLocation` (`self.StaticMeshComponent0`) (.location (`KismetMathLibrary.TLerp` (`self.DownPos`) (`self.UpPos`) _blend)) false false))
      (:`Finished`
        (switch `ETimelineDirection` _direction
          (:`Forward`
            (`KismetSystemLibrary.Delay` 0.5)
            (goto _label :!via `ReverseFromEnd`))
          (:`Backward`
            (`KismetSystemLibrary.Delay` 0.5)
            (goto _label :!via `PlayFromStart`)))))
    (else
      (`SceneComponent.K2_SetWorldLocation` (`self.StaticMeshComponent0`) (.location (`self.UpPos`)) false false)
      (bind (_direction_2 _blend_2) (`Timeline|Timeline` :!label _label_2)
        (:`Update`
          (`SceneComponent.K2_SetWorldLocation` (`self.StaticMeshComponent0`) (.location (`KismetMathLibrary.TLerp` (`self.UpPos`) (`self.DownPos`) _blend_2)) false false))
        (:`Finished`
          (switch `ETimelineDirection` _direction_2
            (:`Forward`
              (`KismetSystemLibrary.Delay` 0.5)
              (goto _label_2 :!via `ReverseFromEnd`))
            (:`Backward`
              (`KismetSystemLibrary.Delay` 0.5)
              (goto _label_2 :!via `PlayFromStart`))))))))

(fn `UserConstructionScript`)