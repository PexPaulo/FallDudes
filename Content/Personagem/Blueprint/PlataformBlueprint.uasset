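; Moving platform Blueprint that shuttles a static mesh back and forth between two transforms, StartPos and FinalPost.
; BeginPlay places the mesh at StartPos and plays the MovePlatform timeline, whose Blend track interpolates the transforms and applies only the resulting world location, without sweep.
; When the timeline finishes, it pauses briefly and replays in the opposite direction, creating an endless ping-pong loop.
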(event `self.ReceiveBeginPlay`
  (`SceneComponent.K2_SetWorldLocation` (`self.StaticMeshComponent0`) (.location (`self.StartPos`)) false false)
  (bind (_direction _blend) (`Timeline|MovePlatform` :!label _label)
    (:`Update`
      (`SceneComponent.K2_SetWorldLocation` (`self.StaticMeshComponent0`) (.location (`KismetMathLibrary.TLerp` (`self.FinalPost`) (`self.StartPos`) _blend)) false false))
    (:`Finished`
      (switch `ETimelineDirection` _direction
        (:`Forward`
          (`KismetSystemLibrary.Delay` 0.3)
          (goto _label :!via `ReverseFromEnd`))
        (:`Backward`
          (`KismetSystemLibrary.Delay` 0.3)
          (goto _label :!via `PlayFromStart`))))))

(fn `UserConstructionScript`)